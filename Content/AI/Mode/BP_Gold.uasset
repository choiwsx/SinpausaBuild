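; BP_Gold is a gold pickup for VR that pops upward on spawn through an impulse on its Sphere and spins around its yaw axis.
; When a BP_MotionController overlaps it, it passes its Gold value to GM_HeroMonster's AddGold.
; It then spawns a small particle burst, plays a coin sound and destroys itself immediately, leaving an unconnected Delay unused.
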(event `self.ReceiveBeginPlay`
  (`PrimitiveComponent.AddImpulse` (`self.Sphere`) (* (`self.GetActorUpVector`) 150.0) "None" false))

(event `self.ReceiveTick`
  (params (DeltaSeconds :type "Float (single-precision)"))
  (`self.K2_AddActorLocalRotation` (`KismetMathLibrary.MakeRotator` 0.0 0.0 (* DeltaSeconds (`self.RotationSpeed`)))))

(event `self.ReceiveActorBeginOverlap`
  (params (OtherActor :type "Actor Object Reference"))
  (bind _returnvalue (`self.K2_GetActorLocation`))
  (cast `/Game/VirtualRealityBP/Blueprints/BP_MotionController` OtherActor)
  (bind _asgm_hero_monster (cast `/Game/AI/GM_HeroMonster` (`GameplayStatics.GetGameMode`)))
  (`/Game/AI/GM_HeroMonster.AddGold` _asgm_hero_monster (`self.Gold`))
  (`|ExecutionSequence`
    (:`then_0`
      (`GameplayStatics.SpawnEmitterAtLocation` "/Game/GabrielAguiarProd/ToonProjectilesVol1/Particles/Muzzles/P_GainGold.P_GainGold" _returnvalue (struct) (0.1 0.1 0.1))
      (`GameplayStatics.PlaySoundAtLocation` "/Game/Sound/Using/GameEffectSound/Coins_10.Coins_10" _returnvalue (struct) 1.0 1.0 0.0 null null null)
      (`self.K2_DestroyActor`))))

(fn `UserConstructionScript`)
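; Tower-defense game mode (tutorial variant, by name) running monster waves, gold and stage progression.
; BeginPlay reads stage gold, life and wave count from DataTables and starts a looping timer spawning the current wave's monsters onto the first spline.
; CheckMonsterCount advances waves once no monsters remain, then fades to the next stage's map or, after the last, the start menu.
; It also refreshes build/upgrade widgets on gold changes and respawns heroes from graves.
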(event `NextWave`
  (set `self.MonsterCount` 0)
  (`|ExecutionSequence`
    (:`then_1`
      (bind _outactors (`GameplayStatics.GetAllActorsOfClass` "/Game/AI/Hero/BP_HERO_BASE.BP_HERO_BASE_C"))
      (for _array_element _outactors
        (`KismetArrayLibrary.Array_Clear` (`/Game/AI/Hero/BP_HERO_BASE.BattleMonsterArray` _array_element))))
    (:`then_2`
      (bind _outactors_2 (`GameplayStatics.GetAllActorsOfClass` "/Game/AI/Monster/Spline_Base.Spline_Base_C" :!label _label))
      (`/Engine/EditorBlueprintResources/StandardMacros.IsValid` (`|GetArrayItem` _outactors_2)
        (:`Is Valid`
          (bind _returnvalue (`KismetSystemLibrary.K2_SetTimerDelegate` (delegate `SpawnMonster`) 1.0 true))
          (set `self.SpawnEvent` _returnvalue))))))

(event `self.ReceiveBeginPlay`
  (`|ExecutionSequence`
    (:`then_0`
      (goto _label))
    (:`then_1`
      (bind _ashero_monster_game_instance (cast `/Game/AI/HeroMonster_GameInstance` (`GameplayStatics.GetGameInstance`)))
      (bind _returnvalue (`|GetDataTableRow` "/Game/AI/Mode/DT_StageGold.DT_StageGold" (`KismetStringLibrary.Conv_StringToName` (`KismetStringLibrary.Conv_IntToString` (`/Game/AI/HeroMonster_GameInstance.Stage` _ashero_monster_game_instance))))
        (:`then`
          (bind (_stage _gold _life) (break `/Game/AI/Mode/ST_StageGold` _returnvalue))
          (set `self.Gold` _gold)
          (set `self.Life` _life))))
    (:`then_2`
      (bind _ashero_monster_game_instance_2 (cast `/Game/AI/HeroMonster_GameInstance` (`GameplayStatics.GetGameInstance`)))
      (bind _returnvalue_2 (`|GetDataTableRow` "/Game/AI/Monster/DT_StageMonster.DT_StageMonster" (`KismetStringLibrary.Conv_StringToName` (`KismetStringLibrary.Conv_IntToString` (`/Game/AI/HeroMonster_GameInstance.Stage` _ashero_monster_game_instance_2))))
        (:`then`
          (set `self.TotalWave` (`KismetArrayLibrary.Array_Length` (`.Wave_Monster_7_0DB8247948295682E31AD8ACEE019C51` (break `/Game/AI/Monster/ST_Stage` _returnvalue_2)))))))
    (:`then_3`
      (bind _outactors (`GameplayStatics.GetAllActorsOfClass` "/Game/Maps/BP_TeleportLocation.BP_TeleportLocation_C"))
      (set `self.TeleportArray` _outactors))))

(event `SpawnMonster`
  (`self.Server_Spawn`))

(event `Server_Spawn`
  (bind _ashero_monster_game_instance (cast `/Game/AI/HeroMonster_GameInstance` (`GameplayStatics.GetGameInstance`)))
  (bind _returnvalue (`|GetDataTableRow` "/Game/AI/Monster/DT_StageMonster.DT_StageMonster" (`KismetStringLibrary.Conv_StringToName` (`KismetStringLibrary.Conv_IntToString` (`/Game/AI/HeroMonster_GameInstance.Stage` _ashero_monster_game_instance))))
    (:`then`
      (for _array_element (`.Wave_Monster_7_0DB8247948295682E31AD8ACEE019C51` (break `/Game/AI/Monster/ST_Stage` _returnvalue))
        (bind (_wave _monstercount _monster) (break `/Game/AI/Monster/ST_DATA` _array_element))
        (if (== _wave (`self.Wave`))
          (bind _output (`|GetArrayItem` (stale `NextWave` _outactors_2)))
          (bind _returnvalue_2 (`|SpawnActorFromClass` _monster (`self.GetTransform` _output) "AlwaysSpawn" "OverrideRootScale" null null))
          (bind _asbp_monster_basic (cast `/Game/AI/Monster/BP_Monster_BASIC` _returnvalue_2))
          (set `/Game/AI/Monster/BP_Monster_BASIC.Spline_Ref` _output _asbp_monster_basic)
          (`/Engine/EditorBlueprintResources/StandardMacros.IncrementInt` (`self.MonsterCount`)
            (:`  `
              (if (not (< (`self.MonsterCount`) _monstercount))
                (`KismetSystemLibrary.K2_ClearAndInvalidateTimerHandle` (`self.SpawnEvent`))))))))))

(event `AddGold`
  (params (Gold :type Integer))
  (set `self.Gold` (+ Gold (`self.Gold`)))
  (`|ExecutionSequence`
    (:`then_0`
      (bind _outactors (`GameplayStatics.GetAllActorsOfClass` "/Game/AI/Build/Widget/BP_BuildWidget.BP_BuildWidget_C"))
      (for _array_element _outactors
        (`/Engine/EditorBlueprintResources/StandardMacros.IsValid` _array_element
          (:`Is Valid`
            (bind _aswidget_build (cast `/Game/AI/Build/Widget/Widget_Build` (`WidgetComponent.GetUserWidgetObject` (`/Game/AI/Build/Widget/BP_BuildWidget.Widget` _array_element))))
            (`/Engine/EditorBlueprintResources/StandardMacros.IsValid` _aswidget_build
              (:`Is Valid`
                (`/Game/AI/Build/Widget/Widget_Build.Refresh` _aswidget_build)))))))
    (:`then_1`
      (bind _outactors_2 (`GameplayStatics.GetAllActorsOfClass` "/Game/AI/Build/Widget/BP_TowerUpgrade.BP_TowerUpgrade_C"))
      (for _array_element_2 _outactors_2
        (`/Engine/EditorBlueprintResources/StandardMacros.IsValid` _array_element_2
          (:`Is Valid`
            (bind _aswidget_tower_upgrade (cast `/Game/AI/Build/Widget/Widget_TowerUpgrade` (`WidgetComponent.GetUserWidgetObject` (`/Game/AI/Build/Widget/BP_TowerUpgrade.Widget` _array_element_2))))
            (`/Engine/EditorBlueprintResources/StandardMacros.IsValid` _aswidget_tower_upgrade
              (:`Is Valid`
                (`/Game/AI/Build/Widget/Widget_TowerUpgrade.Refresh` _aswidget_tower_upgrade)))))))))

(event `CheckMonsterCount`
  (bind _returnvalue (`GameplayStatics.GetGameInstance`))
  ;[1 1 1] 체크 몬스터
  (bind _outactors (`GameplayStatics.GetAllActorsOfClass` "/Game/AI/Monster/BP_Monster_BASIC.BP_Monster_BASIC_C"))
  (if (== (`KismetArrayLibrary.Array_Length` _outactors) 0)
    (set `self.Wave` (`KismetMathLibrary.Clamp` (+ (`self.Wave`) 1) 0 (`self.TotalWave`)))
    (if (< (`self.Wave`) (`self.TotalWave`))
      (`self.NextWave`)
      (else
        (bind _outactors_2 (`GameplayStatics.GetAllActorsOfClass` "/Script/Engine.TargetPoint"))
        (`|SpawnActorFromClass` "/Game/AI/Mode/BP_StageParticle.BP_StageParticle_C" (`KismetMathLibrary.MakeTransform` (`self.K2_GetActorLocation` (`|GetArrayItem` _outactors_2)) (struct :`Pitch` 90.0)) "Undefined" "OverrideRootScale" null null)
        (`GameplayStatics.PlaySound2D` "/Game/Sound/Using/GameEffectSound/Win.Win" 1.0 1.0 0.0 null null)
        (`PlayerCameraManager.StartCameraFade` (`GameplayStatics.GetPlayerCameraManager` 0) 0.0 1.0 2.0 (`self.NextStageFade`) false false)
        (`KismetSystemLibrary.Delay` 2.0)
        (bind _ashero_monster_game_instance (cast `/Game/AI/HeroMonster_GameInstance` _returnvalue))
        (bind _stage (`/Game/AI/HeroMonster_GameInstance.Stage` _ashero_monster_game_instance))
        (set `/Game/AI/HeroMonster_GameInstance.Stage` (+ _stage 1) _ashero_monster_game_instance)
        (if (== _stage 3)
          (`KismetSystemLibrary.PrintString` "모든 스테이지 클리어!!!")
          (bind _ashero_monster_game_instance_2 (cast `/Game/AI/HeroMonster_GameInstance` _returnvalue))
          (`KismetSystemLibrary.Delay` 2.0)
          (`GameplayStatics.OpenLevel` "StartMenuTest2")
          (set `/Game/AI/HeroMonster_GameInstance.Stage` 0 _ashero_monster_game_instance_2)
          (else
            (bind _returnvalue_2 (`|GetDataTableRow` "/Game/AI/Monster/DT_StageMonster.DT_StageMonster" (`KismetStringLibrary.Conv_StringToName` (`KismetStringLibrary.Conv_IntToString` _stage)))
              (:`then`
                (`GameplayStatics.OpenLevel` (`.MapName_10_3FD76A324326C6931BE7B88683CA0145` (break `/Game/AI/Monster/ST_Stage` _returnvalue_2)))))))))))

(event `Grave_Recovery`
  (params (Location :type "Transform Structure") (Grave :type "/Game/AI/Build/BP_Grave Object Reference") (HeroOwnerTower :type "/Game/BluePrints/AllTower/BP_TowerBase Object Reference"))
  (set `self.Hero` (`/Game/AI/Build/BP_Grave.HeroClass` Grave))
  (set `self.Location` Location)
  (set `self.HeroOwnerTower` HeroOwnerTower)
  (set `self.Grave` Grave)
  (`self.K2_DestroyActor` Grave)
  (`self.Spawn_Hero` (`self.Location`) (`self.Hero`) HeroOwnerTower))

(event `Spawn_Hero`
  (params (NewParam :type "Transform Structure") (NewParam2 :type "/Game/AI/Hero/BP_HERO_BASE Class Reference") (NewParam3 :type "/Game/BluePrints/AllTower/BP_TowerBase Object Reference"))
  (bind _returnvalue (`|SpawnActorFromClass` NewParam2 NewParam "AlwaysSpawn" "OverrideRootScale" null null NewParam3 null))
  (`/Engine/EditorBlueprintResources/StandardMacros.IsValid` NewParam3
    (:`Is Valid`
      (set `/Game/BluePrints/AllTower/BP_TowerBase.Hero` _returnvalue NewParam3))))

(fn `UserConstructionScript`)
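; Base hero AI character that fights monsters and can be picked up and dropped by motion controller.
; SetState syncs Peace, Chase, Attack, Dead and Grab to the Blackboard, setting walk speed and random attack montages.
; Sphere overlap, damage, landing and attack completion trigger nearest-monster targeting; BasicAttack capsule-traces to damage and knock back monsters.
; Damage updates the HP widget; death releases tracked monsters, plays a montage and leaves a grave.
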(event `self.ReceiveBeginPlay`
  ;[1 1 1] 비긴플레이 이벤트
  (`parent.ReceiveBeginPlay`)
  (set `self.CurrentHP` (`self.MaxHP`))
  (`self.SetState` "NewEnumerator0")
  (bind _aswidget_hero_hp (cast `/Game/AI/Hero/Widget/Widget_HeroHP` (`WidgetComponent.GetUserWidgetObject` (`self.HP`))))
  (`ProgressBar.SetPercent` (`/Game/AI/Hero/Widget/Widget_HeroHP.HeroHP` _aswidget_hero_hp) (/ (`self.CurrentHP`) 100.0))
  (`TextBlock.SetText` (`/Game/AI/Hero/Widget/Widget_HeroHP.HeroLevel` _aswidget_hero_hp) (`KismetTextLibrary.Conv_IntToText` (`self.Level`)))
  (`SceneComponent.SetVisibility` (`self.Recovery`) false false))

(event `self.ReceiveTick`
  (params (DeltaSeconds :type "Float (single-precision)"))
  ;[1 1 1] Tick 이벤트
  (`parent.ReceiveTick` DeltaSeconds)
  (`|ExecutionSequence`))

(event `/Game/VirtualRealityBP/Blueprints/PickupActorInterface.Pickup`
  (params (AttachTo :type "SceneComponent Object Reference") (Rotator :type "Rotator Structure"))
  ;[1 1 1] 모션컨트롤러 PickUP & Drop 이벤트
  (set `self.ActorRotator` Rotator)
  (`SceneComponent.K2_AttachToComponent` (`self.CapsuleComponent`) AttachTo "None" "KeepWorld" "KeepWorld" "KeepWorld" false)
  (set `CharacterMovementComponent.GravityScale` 0.0 (`self.CharacterMovement`))
  (`PrimitiveComponent.SetCollisionEnabled` (`self.CapsuleComponent`) "NoCollision")
  (`self.SetState` "NewEnumerator4")
  (set `self.Instigator` null)
  (for _array_element (`self.Monsters`)
    (`/Engine/EditorBlueprintResources/StandardMacros.IsValid` _array_element
      (:`Is Valid`
        (`/Game/AI/Monster/BP_Monster_BASIC.SetState` _array_element "NewEnumerator0")
        (set `Actor.Instigator` null _array_element)
        (set `/Game/AI/Monster/BP_Monster_BASIC.TargetHero` null _array_element)
        (`/Game/AI/Monster/BP_Monster_BASIC.Initi_TargetLoc` _array_element))))
  (`KismetArrayLibrary.Array_Clear` (`self.Monsters`)))

(event `PickupServer`
  (params (NewParam :type "SceneComponent Object Reference") (NewParam2 :type "Rotator Structure"))
  ;[1 1 1] 모션컨트롤러 PickUP & Drop 이벤트
)

(event `/Game/VirtualRealityBP/Blueprints/PickupActorInterface.Drop`
  ;[1 1 1] 모션컨트롤러 PickUP & Drop 이벤트
  (`PrimitiveComponent.SetCollisionEnabled` (`self.CapsuleComponent`) "QueryAndPhysics")
  (`SceneComponent.K2_DetachFromComponent` (`self.CapsuleComponent`) "KeepWorld" "KeepWorld" "KeepWorld" true)
  (set `CharacterMovementComponent.GravityScale` 1.0 (`self.CharacterMovement`))
  (set `self.Instigator` null)
  (bind _returnvalue (`KismetSystemLibrary.K2_SetTimerDelegate` (delegate `DropHero`) 0.1 true))
  (set `self.FallingEvent` _returnvalue))

(event `DropHero`
  ;[1 1 1] 모션컨트롤러 PickUP & Drop 이벤트
  (if (not (`NavMovementComponent.IsFalling` (`self.CharacterMovement`)))
    (`self.K2_SetActorRotation` (`self.ActorRotator`))
    (`self.SetState` "NewEnumerator0")
    (`self.AggroCheck`)
    (`KismetSystemLibrary.K2_ClearAndInvalidateTimerHandle` (`self.FallingEvent`))))

(event `Reset_MonsterInformation`
  (bind (_returnvalue_location _returnvalue_rotation) (`KismetMathLibrary.BreakTransform` (`self.GetTransform`)))
  (for _array_element (`self.Monsters`)
    (`/Engine/EditorBlueprintResources/StandardMacros.IsValid` _array_element
      (:`Is Valid`
        (`/Game/AI/Monster/BP_Monster_BASIC.SetState` _array_element "NewEnumerator6")
        (set `Actor.Instigator` null _array_element)
        (set `/Game/AI/Monster/BP_Monster_BASIC.TargetHero` null _array_element)
        (`/Game/AI/Monster/BP_Monster_BASIC.Initi_TargetLoc` _array_element))))
  (`KismetArrayLibrary.Array_Clear` (`self.Monsters`))
  (`|PlayMontage` (`self.SkeletalMesh1`) (`self.Die_Montage`) 2.0 0.0 (`KismetStringLibrary.Conv_StringToName` (`KismetTextLibrary.Conv_TextToString` (`|FormatText` "Death{number}" (`KismetMathLibrary.RandomIntegerInRange` 1 5))))
    (:`then`
      (`self.SetActorEnableCollision` false)
      (`PrimitiveComponent.SetCollisionEnabled` (`self.CapsuleComponent`) "NoCollision"))
    (:`OnCompleted`
      (`|SpawnActorFromClass` "/Game/AI/Build/BP_Grave.BP_Grave_C" (`KismetMathLibrary.MakeTransform` _returnvalue_location _returnvalue_rotation (1.0 1.0 1.0)) "AlwaysSpawn" "OverrideRootScale" null null)
      (`self.K2_DestroyActor`))))

(event `self.ReceiveAnyDamage`
  (params (Damage :type "Float (single-precision)") (DamageType :type "DamageType Object Reference") (InstigatedBy :type "Controller Object Reference") (DamageCauser :type "Actor Object Reference"))
  ;[1 1 1] AnyDamage 이벤트
  (`self.AggroCheck`)
  (bind _output_get (set `self.CurrentHP` (- (`self.CurrentHP`) Damage)))
  (bind _aswidget_hero_hp (cast `/Game/AI/Hero/Widget/Widget_HeroHP` (`WidgetComponent.GetUserWidgetObject` (`self.HP`))))
  (`ProgressBar.SetPercent` (`/Game/AI/Hero/Widget/Widget_HeroHP.HeroHP` _aswidget_hero_hp) (/ (`self.CurrentHP`) 100.0))
  (if (not (> _output_get 0.0))
    (`self.SetState` "NewEnumerator3")
    (`self.Reset_MonsterInformation`)))

(event `SetState`
  (params (NewState :type "/Game/AI/Hero/BPE_HeroState Enum" :default "NewEnumerator0"))
  (bind _returnvalue (`AIBlueprintHelperLibrary.GetBlackboard` (`self.GetController`)))
  ;[1 1 1] SetState 이벤트
  (if (`|EnumInequality` (`self.CurrentStatePawn`) "NewEnumerator3")
    (bind _output_get (set `self.CurrentStatePawn` NewState))
    (`|ExecutionSequence`
      (:`then_0`
        (`/Engine/EditorBlueprintResources/StandardMacros.IsValid` _returnvalue
          (:`Is Valid`
            (`BlackboardComponent.SetValueAsEnum` _returnvalue (`self.StateKey`) _output_get))))
      (:`then_1`
        (switch `/Game/AI/Hero/BPE_HeroState` (`self.CurrentStatePawn`)
          (:`NewEnumerator0`
            (set `CharacterMovementComponent.MaxWalkSpeed` 5.0 (`self.CharacterMovement`)))
          (:`NewEnumerator1`
            (set `CharacterMovementComponent.MaxWalkSpeed` 20.0 (`self.CharacterMovement`)))
          (:`NewEnumerator2`
            (set `CharacterMovementComponent.MaxWalkSpeed` 0.0 (`self.CharacterMovement`))
            (`self.LookTargetMonster` (`self.TargetMonster`))
            (`/Engine/EditorBlueprintResources/StandardMacros.IsValid` (`self.BaiscAttack_Montage`)
              (:`Is Valid`
                (`|PlayMontage` (`self.SkeletalMesh1`) (`self.BaiscAttack_Montage`) 1.0 0.0 (`KismetStringLibrary.Conv_StringToName` (`KismetTextLibrary.Conv_TextToString` (`|FormatText` "Attack{Num}" (`KismetMathLibrary.RandomIntegerInRange` 1 (`self.Int_BasicAttackMontageCount`)))))
                  (:`OnCompleted`
                    (if (`|EnumInequality` (`self.CurrentStatePawn`) "NewEnumerator4")
                      (`self.AggroCheck`)))))))
          (:`NewEnumerator3`
            (set `CharacterMovementComponent.MaxWalkSpeed` 0.0 (`self.CharacterMovement`)))
          (:`NewEnumerator4`
            (set `CharacterMovementComponent.MaxWalkSpeed` 0.0 (`self.CharacterMovement`))
            (set `self.Instigator` null)))))))

(event `LookTargetMonster`
  (params (TargetMonster :type "/Game/AI/Monster/BP_Monster_BASIC Object Reference"))
  (bind (_returnvalue_roll _returnvalue_pitch _returnvalue_yaw) (`KismetMathLibrary.BreakRotator` (`KismetMathLibrary.FindLookAtRotation` (`self.K2_GetActorLocation`) (`self.K2_GetActorLocation` TargetMonster))))
  ;[1 1 1] 몬스터 바라보기
  (`/Engine/EditorBlueprintResources/StandardMacros.IsValid` TargetMonster
    (:`Is Valid`
      (`self.K2_SetActorRotation` (`KismetMathLibrary.MakeRotator` 0.0 0.0 _returnvalue_yaw)))))

(event `self.PawnSensing.OnSeePawn`
  (params (Pawn :type "Pawn Object Reference"))
  ;[1 1 1] OnSeePawn이벤트
)

(event `BasicAttack`
  (params (Damage :type "Float (double-precision)"))
  (bind _returnvalue (`self.K2_GetActorLocation`))
  ;[1 1 1] 공격애님파이에 따른 이벤트
  (bind _outactors (`GameplayStatics.GetAllActorsOfClass` "BP_HERO_BASE_C"))
  (bind _outhit (`KismetSystemLibrary.CapsuleTraceSingleForObjects` _returnvalue (+ _returnvalue (* (`self.GetActorForwardVector`) 6.0)) 8.0 5.0 (`|MakeArray` "ObjectTypeQuery3" :!type "EObjectTypeQuery Enum") false _outactors "ForDuration"))
  (bind (_bblockinghit _binitialoverlap _time _distance _location _impactpoint _normal _impactnormal _physmat _hitactor) (`GameplayStatics.BreakHitResult` _outhit))
  (bind _asbp_monster_basic (cast `/Game/AI/Monster/BP_Monster_BASIC` _hitactor))
  (`/Engine/EditorBlueprintResources/StandardMacros.IsValid` _asbp_monster_basic
    (:`Is Valid`
      (`CharacterMovementComponent.AddImpulse` (`Character.CharacterMovement` _asbp_monster_basic) (* (`self.GetActorForwardVector` _asbp_monster_basic) -200.0) false)
      (bind _returnvalue_2 (`GameplayStatics.SpawnEmitterAtLocation` "/Game/SimpleCartoonFX/FX/Hit2.Hit2" _impactpoint (struct) (0.05 0.05 0.05)))
      (set `self.HitEmitter` _returnvalue_2)
      (`GameplayStatics.PlaySoundAtLocation` "/Game/Sound/Using/HeroSound/SwordAction.SwordAction" _impactpoint (struct) 1.0 1.0 0.0 null null null)
      (`GameplayStatics.ApplyDamage` _asbp_monster_basic Damage null self))))

(event `AggroCheck`
  (bind _targetmonster (`self.TargetMonster`))
  ;[1 1 1] 어그로 체크(영웅 액터와 가장 가까운 몬스터 찾기)
  (set `self.DistanceToMonster` (`self.CheckDistanceToMonster`))
  (set `self.TargetMonster` null)
  (bind _outactors (`GameplayStatics.GetAllActorsOfClass` "/Game/AI/Monster/BP_Monster_BASIC.BP_Monster_BASIC_C"))
  (for _array_element _outactors
    (bind _returnvalue (`KismetMathLibrary.VSize` (- (`self.K2_GetActorLocation` _array_element) (`self.K2_GetActorLocation`))))
    (if (< _returnvalue (`self.DistanceToMonster`))
      (set `self.DistanceToMonster` _returnvalue)
      (set `self.TargetMonster` _array_element)))
  (`/Engine/EditorBlueprintResources/StandardMacros.IsValid` _targetmonster
    (:`Is Valid`
      (set `self.Instigator` _targetmonster)
      (`self.SetState` "NewEnumerator1")
      (if (< (`KismetArrayLibrary.Array_Length` (`self.BattleMonsterArray`)) (`self.BattleMonsterCount`))
        (`KismetArrayLibrary.Array_AddUnique` (`self.BattleMonsterArray`) (`self.TargetMonster`))))))

(event `self.Sphere.OnComponentBeginOverlap`
  (params (OverlappedComponent :type "PrimitiveComponent Object Reference") (OtherActor :type "Actor Object Reference") (OtherComp :type "PrimitiveComponent Object Reference") (OtherBodyIndex :type Integer) (bFromSweep :type Boolean) (SweepResult :type "HitResult Structure (by ref)"))
  (bind _targetmonster (`self.TargetMonster`))
  ;[1 1 1] Sphere Collision 을 이용해서 주변 적 발견하기
  (`|ExecutionSequence`
    (:`then_0`
      (bind _asbp_monster_basic (cast `/Game/AI/Monster/BP_Monster_BASIC` OtherActor))
      (set `self.DistanceToMonster` (`self.CheckDistanceToMonster`))
      (set `self.TargetMonster` _asbp_monster_basic)
      (if (`|EnumInequality` (`self.CurrentStatePawn`) "NewEnumerator4")
        (if (`|EnumEquality` (`self.CurrentStatePawn`) "NewEnumerator0")
          (bind _outactors (`GameplayStatics.GetAllActorsOfClass` "/Game/AI/Monster/BP_Monster_BASIC.BP_Monster_BASIC_C"))
          (for _array_element _outactors
            (bind _returnvalue (`KismetMathLibrary.VSize` (- (`self.K2_GetActorLocation` _array_element) (`self.K2_GetActorLocation`))))
            (if (< _returnvalue (`self.DistanceToMonster`))
              (set `self.DistanceToMonster` _returnvalue)
              (set `self.TargetMonster` _array_element)))
          (`/Engine/EditorBlueprintResources/StandardMacros.IsValid` _targetmonster
            (:`Is Valid`
              (set `self.Instigator` _targetmonster)
              (`self.SetState` "NewEnumerator1")
              (if (< (`KismetArrayLibrary.Array_Length` (`self.BattleMonsterArray`)) (`self.BattleMonsterCount`))
                (`KismetArrayLibrary.Array_AddUnique` (`self.BattleMonsterArray`) (`self.TargetMonster`))))))))
    (:`then_1`
      (cast `/Game/VirtualRealityBP/Blueprints/BP_MotionController` OtherActor))))

(event `RemoveBattleMonster`
  (params (Monster :type "/Game/AI/Monster/BP_Monster_BASIC Object Reference"))
  (`/Engine/EditorBlueprintResources/StandardMacros.IsValid` Monster
    (:`Is Valid`
      (`KismetArrayLibrary.Array_RemoveItem` (`self.BattleMonsterArray`) Monster))))

(event `Attack_S_Move`
  (set `CharacterMovementComponent.MaxWalkSpeed` 0.0 (`self.CharacterMovement`)))

(event `Attack_E_Move`
  (set `CharacterMovementComponent.MaxWalkSpeed` 600.0 (`self.CharacterMovement`)))

(fn `UserConstructionScript`
  (`parent.UserConstructionScript`))
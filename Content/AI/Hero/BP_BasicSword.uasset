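; Sword hero Blueprint whose stats and modular gear follow its level, extending a parent hero class.
; On BeginPlay, body-part meshes follow the main skeletal mesh via master pose, and base damage comes from a data table row keyed by Level.
; HeroLevelUp rereads that table to refill HP, update damage and attack montage count, swap gear meshes and refresh the HP widget.
; Tick destroys the hero once its BaseTower is invalid.
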(event `self.ReceiveBeginPlay`
  (`parent.ReceiveBeginPlay`)
  (`SkinnedMeshComponent.SetLeaderPoseComponent` (`self.Face`) (`self.SkeletalMesh1`) false)
  (`SkinnedMeshComponent.SetLeaderPoseComponent` (`self.Hair`) (`self.SkeletalMesh1`) false)
  (`SkinnedMeshComponent.SetLeaderPoseComponent` (`self.Glove`) (`self.SkeletalMesh1`) false)
  (`SkinnedMeshComponent.SetLeaderPoseComponent` (`self.HeadGears`) (`self.SkeletalMesh1`) false)
  (`SkinnedMeshComponent.SetLeaderPoseComponent` (`self.Belt`) (`self.SkeletalMesh1`) false)
  (`SkinnedMeshComponent.SetLeaderPoseComponent` (`self.Shoe`) (`self.SkeletalMesh1`) false)
  (bind _returnvalue (`|GetDataTableRow` (`self.StructTable`) (`KismetStringLibrary.Conv_StringToName` (`KismetStringLibrary.Conv_IntToString` (`self.Level`))))
    (:`then`
      (set `self.BasicDamage` (`.BasicDamage_7_4D3C87E343836B47A3F5969C2BAA36D5` (break `/Game/AI/Hero/Struct/ST_Hero` _returnvalue))))))

(event `HideSkeletalMesh_1`)

(event `HeroLevelUp`
  (bind _aswidget_hero_hp (cast `/Game/AI/Hero/Widget/Widget_HeroHP` (`WidgetComponent.GetUserWidgetObject` (`self.HP`))))
  (bind _returnvalue (`|GetDataTableRow` (`self.StructTable`) (`KismetStringLibrary.Conv_StringToName` (`KismetStringLibrary.Conv_IntToString` (`self.Level`))))
    (:`then`
      (bind (_level _maxhp _basicdamage _attackmontagecount _glove _headgears _hair _belt _shoe) (break `/Game/AI/Hero/Struct/ST_Hero` _returnvalue))
      (bind _output_get (set `self.MaxHP` _maxhp))
      (set `self.CurrentHP` _output_get)
      (set `self.BasicDamage` _basicdamage)
      (set `self.Int_BasicAttackMontageCount` _attackmontagecount)
      (`SkinnedMeshComponent.SetSkinnedAssetAndUpdate` (`self.Glove`) _glove false)
      (`SkinnedMeshComponent.SetSkinnedAssetAndUpdate` (`self.HeadGears`) _headgears true)
      (`SkinnedMeshComponent.SetSkinnedAssetAndUpdate` (`self.Hair`) _hair true)
      (`SkinnedMeshComponent.SetSkinnedAssetAndUpdate` (`self.Belt`) _belt true)
      (`SkinnedMeshComponent.SetSkinnedAssetAndUpdate` (`self.Shoe`) _shoe true)
      (`ProgressBar.SetPercent` (`/Game/AI/Hero/Widget/Widget_HeroHP.HeroHP` _aswidget_hero_hp) (/ (`self.CurrentHP`) 100.0))
      (`TextBlock.SetText` (`/Game/AI/Hero/Widget/Widget_HeroHP.HeroLevel` _aswidget_hero_hp) (`KismetTextLibrary.Conv_IntToText` (`self.Level`))))))

(event `self.ReceiveTick`
  (params (DeltaSeconds :type "Float (single-precision)"))
  (`parent.ReceiveTick` DeltaSeconds)
  (`/Engine/EditorBlueprintResources/StandardMacros.IsValid` (`self.BaseTower`)
    (:`Is Not Valid`
      (`self.K2_DestroyActor`))))

(fn `UserConstructionScript`
  (`parent.UserConstructionScript`))
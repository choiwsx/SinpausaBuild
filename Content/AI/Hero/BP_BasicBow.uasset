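; BP_BasicBow is a bow-wielding hero Blueprint under AI/Hero that adds arrow firing to its parent class.
; ArrowSpawn plays a small muzzle particle, spawns an owned ArrowActor along the actor's rotation and plays an arrow sound, all at the left-hand bow socket.
; Tick only calls the parent, HideSkeletalMesh_2 is empty, and a node hiding the Bow component is disconnected.
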(event `HideSkeletalMesh_2`)

(event `self.ReceiveTick`
  (params (DeltaSeconds :type "Float (single-precision)"))
  (`parent.ReceiveTick` DeltaSeconds))

(event `ArrowSpawn`
  (bind _returnvalue (`SceneComponent.GetSocketLocation` (`self.SkeletalMesh1`) "hand_lBowSocket"))
  (`GameplayStatics.SpawnEmitterAtLocation` "/Game/GabrielAguiarProd/ToonProjectilesVol1/Particles/Muzzles/P_Muzzle_Bullet01Lowpoly.P_Muzzle_Bullet01Lowpoly" (`SceneComponent.GetSocketLocation` (`self.SkeletalMesh1`) "hand_lBowSocket") (`self.K2_GetActorRotation`) (0.05 0.05 0.05))
  (`|SpawnActorFromClass` (`self.ArrowActor`) (`KismetMathLibrary.MakeTransform` _returnvalue (`self.K2_GetActorRotation`)) "AlwaysSpawn" "OverrideRootScale" self null)
  (`GameplayStatics.PlaySoundAtLocation` "/Game/Sound/Using/TowerAttackSound/Arrow_Impact_flesh__human__8.Arrow_Impact_flesh__human__8" _returnvalue (struct) 1.0 1.0 0.0 null null null))

(fn `UserConstructionScript`
  (`parent.UserConstructionScript`))
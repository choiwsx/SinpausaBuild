(event `self.ReceiveBeginPlay`)

(event `Key|Five`
  (params (Key :type "Key Structure"))
  (:`Pressed`
    (bind _outactors (`GameplayStatics.GetAllActorsOfClass` "/Game/AI/Hero/BP_BasicSword.BP_BasicSword_C"))
    (for _array_element _outactors
      (`/Engine/EditorBlueprintResources/StandardMacros.IncrementInt` (`/Game/AI/Hero/BP_HERO_BASE.Level` _array_element)
        (:`  `
          (`/Game/AI/Hero/BP_BasicSword.HeroLevelUp` _array_element))))))

(event `Server_TowerSelected`
  (params (NewParam :type "/Game/BluePrints/AllTower/BP_TowerSelect Object Reference"))
  (bind _output_get (set `self.Tower_Selected` NewParam))
  (`KismetSystemLibrary.PrintString` (`KismetSystemLibrary.GetDisplayName` _output_get)))

(event `Server_Upgrade`
  (params (NewParam :type Integer) (NewParam2 :type "Transform Structure") (NewParam3 :type "/Game/BluePrints/AllTower/BP_TowerBase Object Reference"))
  (bind _returnvalue (`KismetStringLibrary.Conv_StringToName` (`KismetStringLibrary.Conv_IntToString` NewParam)))
  (bind _returnvalue_2 (`|GetDataTableRow` "/Game/HR/BP_HRDataTable.BP_HRDataTable" _returnvalue)
    (:`then`
      (bind (_towernumber _towername _towerattackdelay _towerdamage _towerange _towerselection _attacktype _magictype _needgold) (break `/Game/HR/BP_HRStruct` _returnvalue_2))
      (bind _returnvalue_3 (`|SpawnActorFromClass` _towerselection NewParam2 "AlwaysSpawn" "OverrideRootScale" null _returnvalue null))
      (`/Engine/EditorBlueprintResources/StandardMacros.IsValid` _returnvalue_3
        (:`Is Valid`
          (`/Engine/EditorBlueprintResources/StandardMacros.IsValid` NewParam3
            (:`Is Valid`
              (`self.K2_DestroyActor` NewParam3)
              (bind _asgm_hero_monster (cast `/Game/AI/GM_HeroMonster` (`GameplayStatics.GetGameMode`)))
              (set `/Game/AI/GM_HeroMonster.Gold` (- (`/Game/AI/GM_HeroMonster.Gold` _asgm_hero_monster) _needgold) _asgm_hero_monster))))))))

(event `Spawn_Tower`
  (params (NewParam :type Integer) (NewParam2 :type "Transform Structure") (NewParam3 :type "/Game/BluePrints/AllTower/BP_TowerAreaWonseok Object Reference"))
  (bind _returnvalue (`KismetStringLibrary.Conv_StringToName` (`KismetStringLibrary.Conv_IntToString` NewParam)))
  (bind _returnvalue_2 (`|GetDataTableRow` "/Game/HR/BP_HRDataTable.BP_HRDataTable" _returnvalue)
    (:`then`
      (bind (_towernumber _towername _towerattackdelay _towerdamage _towerange _towerselection _attacktype _magictype _needgold) (break `/Game/HR/BP_HRStruct` _returnvalue_2))
      (bind _returnvalue_3 (`|SpawnActorFromClass` _towerselection NewParam2 "AlwaysSpawn" "OverrideRootScale" null _returnvalue null))
      (`/Engine/EditorBlueprintResources/StandardMacros.IsValid` _returnvalue_3
        (:`Is Valid`
          (`/Engine/EditorBlueprintResources/StandardMacros.IsValid` NewParam3
            (:`Is Valid`
              (`self.K2_DestroyActor` NewParam3)
              (bind _asgm_hero_monster (cast `/Game/AI/GM_HeroMonster` (`GameplayStatics.GetGameMode`)))
              (set `/Game/AI/GM_HeroMonster.Gold` (- (`/Game/AI/GM_HeroMonster.Gold` _asgm_hero_monster) _needgold) _asgm_hero_monster))))))))

(event `Server_SellSpawn`
  (params (Loc :type "Transform Structure") (TowerBase :type "/Game/BluePrints/AllTower/BP_TowerBase Object Reference"))
  (bind _returnvalue (`|SpawnActorFromClass` "/Game/BluePrints/AllTower/BP_TowerAreaWonseok.BP_TowerAreaWonseok_C" (`KismetMathLibrary.MakeTransform` (.location Loc)) "Undefined" "OverrideRootScale" null null))
  (`/Engine/EditorBlueprintResources/StandardMacros.IsValid` _returnvalue
    (:`Is Valid`
      (`/Engine/EditorBlueprintResources/StandardMacros.IsValid` TowerBase
        (:`Is Valid`
          (`self.K2_DestroyActor` TowerBase))))))

(event `SpawnBow`
  (params (NewParam :type "Vector Structure") (NewParam2 :type "Rotator Structure") (NewParam3 :type "Float (double-precision)"))
  (`|SpawnActorFromClass` "/Game/Heroic_medieval_pack/Props/Bp_Cannon.Bp_Cannon_C" (`KismetMathLibrary.MakeTransform` NewParam NewParam2) "AlwaysSpawn" "OverrideRootScale" null null))

(event `SetPercent`
  (params (NewParam :type "Float (double-precision)") (NewParam2 :type "/Game/AI/Monster/BP_Monster_BASIC Object Reference"))
  (`/Engine/EditorBlueprintResources/ActorMacros.Switch Has Authority`
    (:`Remote`
      (bind _aswidget_monster_hp (cast `/Game/AI/Monster/Widget/Widget_MonsterHP` (`WidgetComponent.GetUserWidgetObject` (`/Game/AI/Monster/BP_Monster_BASIC.Widget` NewParam2))))
      (`ProgressBar.SetPercent` (`/Game/AI/Monster/Widget/Widget_MonsterHP.HP` _aswidget_monster_hp) NewParam))))

(event `Spawn_BuildWidget`
  (params (MotionController :type "/Game/VirtualRealityBP/Blueprints/BP_MotionController Object Reference") (Transform :type "Transform Structure") (TowerBase :type "/Game/BluePrints/AllTower/BP_TowerAreaWonseok Object Reference") (PlayerController :type "/Game/AI/PC_Controller Object Reference"))
  (bind _returnvalue (`|SpawnActorFromClass` "/Game/AI/Build/Widget/BP_BuildWidget.BP_BuildWidget_C" Transform "AlwaysSpawn" "OverrideRootScale" null null))
  (set `self.BuildActor` _returnvalue)
  (bind _buildwidget (`/Game/AI/Build/Widget/BP_BuildWidget.BuildWidget` _returnvalue))
  (`/Engine/EditorBlueprintResources/StandardMacros.IsValid` (`/Game/AI/Build/Widget/Widget_Build.OwnTower` _buildwidget)
    (:`Is Not Valid`
      (set `/Game/AI/Build/Widget/Widget_Build.OwnTower` TowerBase _buildwidget)
      (bind _output_get (set `/Game/AI/Build/Widget/Widget_Build.MotionController` MotionController (`/Game/AI/Build/Widget/BP_BuildWidget.BuildWidget` _returnvalue)))
      (set `/Game/AI/Build/Widget/Widget_Build.PlayController` PlayerController _buildwidget)
      (`ActorComponent.Activate` (`/Game/VirtualRealityBP/Blueprints/BP_MotionController.WidgetInteraction` MotionController) false)
      (bind _asmotion_controller_pawn (cast `/Game/VirtualRealityBP/Blueprints/MotionControllerPawn` (`self.GetOwner` _output_get)))
      (set `/Game/VirtualRealityBP/Blueprints/MotionControllerPawn.IsBuilding?` true _asmotion_controller_pawn))))

(event `Spawn_Upgrade`
  (params (MotionController :type "/Game/VirtualRealityBP/Blueprints/BP_MotionController Object Reference") (Transform :type "Transform Structure") (TowerBase :type "/Game/BluePrints/AllTower/BP_TowerBase Object Reference"))
  (bind _motioncontroller (`self.MotionController`))
  (bind _returnvalue (`|SpawnActorFromClass` "/Game/AI/Build/Widget/BP_TowerUpgrade.BP_TowerUpgrade_C" Transform "AlwaysSpawn" "OverrideRootScale" null null))
  (set `self.UpgradeActor` _returnvalue)
  (set `self.MotionController` MotionController)
  (bind _upgradewidget (`/Game/AI/Build/Widget/BP_TowerUpgrade.UpgradeWidget` _returnvalue))
  (`/Engine/EditorBlueprintResources/StandardMacros.IsValid` (`/Game/AI/Build/Widget/Widget_TowerUpgrade.OwnTower` _upgradewidget)
    (:`Is Not Valid`
      (set `/Game/AI/Build/Widget/Widget_TowerUpgrade.OwnTower` TowerBase _upgradewidget)
      (set `/Game/AI/Build/Widget/Widget_TowerUpgrade.MotionController` _motioncontroller _upgradewidget)
      (`ActorComponent.Activate` (`/Game/VirtualRealityBP/Blueprints/BP_MotionController.WidgetInteraction` _motioncontroller) false)
      (bind _asmotion_controller_pawn (cast `/Game/VirtualRealityBP/Blueprints/MotionControllerPawn` (`self.GetOwner` _motioncontroller)))
      (set `/Game/VirtualRealityBP/Blueprints/MotionControllerPawn.IsBuilding?` true _asmotion_controller_pawn))))

(event `Delete_BuildActor`
  (bind _buildactor (`self.BuildActor`))
  (`/Engine/EditorBlueprintResources/StandardMacros.IsValid` _buildactor
    (:`Is Valid`
      (`self.K2_DestroyActor` _buildactor))
    (:`Is Not Valid`
      (`KismetSystemLibrary.PrintString` "Fail"))))

(event `Delete_Upgrade`
  (bind _upgradeactor (`self.UpgradeActor`))
  (`/Engine/EditorBlueprintResources/StandardMacros.IsValid` _upgradeactor
    (:`Is Valid`
      (`self.K2_DestroyActor` _upgradeactor))
    (:`Is Not Valid`
      (`KismetSystemLibrary.PrintString` "12341234"))))

(fn `UserConstructionScript`)
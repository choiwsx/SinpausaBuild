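; Monster component that applies an ice slow to its owning BP_Monster_BASIC as a secondary damage effect.
; HandleDamage saves the base speed if not already slowed, then multiplies current speed by the damage type's FinalSpeed on every hit.
; A looping one-second timer counts past Duration, then restores speed, clears the particle template and slow flag, and resets the count.
; The timer handle is stored but never cleared here.
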(event `self.ReceiveBeginPlay`
  (bind _asbp_monster_basic (cast `/Game/AI/Monster/BP_Monster_BASIC` (`self.GetOwner`)))
  (set `self.RefMonster` _asbp_monster_basic)
  (bind _aswidget_monster_hp (cast `/Game/AI/Monster/Widget/Widget_MonsterHP` (`WidgetComponent.GetUserWidgetObject` (`/Game/AI/Monster/BP_Monster_BASIC.Widget` (`self.RefMonster`)))))
  (set `self.RefMonsterHP` _aswidget_monster_hp))

(event `self.HandleDamage`
  (params (DamageType :type "/Game/BluePrints/AllTower/MagicTower/DamageType/BP_DamageBase Object Reference") (DamageCauser :type "Actor Object Reference"))
  (bind _refmonster (`self.RefMonster`))
  ;[1 1 1] 2차 데미지 효과 처리
  (bind _output_get (set `self.RefDamageType` DamageType))
  (`/Engine/EditorBlueprintResources/StandardMacros.IsValid` _output_get
    (:`Is Valid`
      (if (not (`/Game/AI/Monster/BP_Monster_BASIC.IsSlow?` _refmonster))
        (set `self.BasicSpeed` (`/Game/AI/Monster/BP_Monster_BASIC.CurrentSpeed` _refmonster))
        (set `/Game/AI/Monster/BP_Monster_BASIC.IsSlow?` true _refmonster))
      (set `/Game/AI/Monster/BP_Monster_BASIC.CurrentSpeed` (* (`/Game/AI/Monster/BP_Monster_BASIC.CurrentSpeed` (`self.RefMonster`)) (`/Game/BluePrints/AllTower/MagicTower/DamageType/BP_DamageBase.FinalSpeed` (`self.RefDamageType`))) (`self.RefMonster`))
      (bind _returnvalue (`KismetSystemLibrary.K2_SetTimerDelegate` (delegate `AfterMainDamage`) 1.0 true))
      (set `self.TimeHandle` _returnvalue))))

(event `AfterMainDamage`
  (bind _refmonster (`self.RefMonster`))
  ;[1 1 1] 2차 데미지 효과 처리
  (`/Engine/EditorBlueprintResources/StandardMacros.IsValid` (`self.RefDamageType`)
    (:`Is Valid`
      (bind _result (`/Engine/EditorBlueprintResources/StandardMacros.IncrementInt` (`self.Count`))
        (:`  `
          (if (> _result (`/Game/BluePrints/AllTower/MagicTower/DamageType/BP_DamageBase.Duration` (`self.RefDamageType`)))
            (set `/Game/AI/Monster/BP_Monster_BASIC.CurrentSpeed` (`self.BasicSpeed`) _refmonster)
            (`ParticleSystemComponent.SetTemplate` (`/Game/AI/Monster/BP_Monster_BASIC.ParticleSystem` _refmonster) null)
            (`self.FinishTimer`)
            (set `/Game/AI/Monster/BP_Monster_BASIC.IsSlow?` false (`self.RefMonster`))))))))

(event `ResetReferences`
  ;[1 1 1] 참조 변수 초기화
  (set `self.RefDamageType` null)
  (set `self.RefDamageCauser` null))

(event `FinishTimer`
  ;[1 1 1] 타이머 종료
  (set `self.Count` 0))
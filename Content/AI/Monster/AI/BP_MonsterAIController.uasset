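; BP_MonsterAIController is the AI controller for a monster, starting its AI when play begins.
; BeginPlay sets up the BB_MonsterAI1 blackboard, then runs the BT_MonsterAI1 behavior tree.
; Disconnected nodes that would write home location, idle time and a random navigable target location to the blackboard never run.
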(event `self.ReceiveBeginPlay`
  (`|ExecutionSequence`
    (:`then_0`
      (`self.UseBlackboard` "/Game/AI/Monster/AI/BB_MonsterAI1.BB_MonsterAI1"))
    (:`then_1`
      (`self.RunBehaviorTree` "/Game/AI/Monster/AI/BT_MonsterAI1.BT_MonsterAI1"))))

(fn `UserConstructionScript`)
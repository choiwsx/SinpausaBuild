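; Monster AI character that walks a spline, chases and attacks nearby heroes, and drops gold on death.
; The server loads stats by Level from DT_Monster and moves it while at peace; PawnSensing and aggro checks pick the nearest hero.
; SetState mirrors the state to the Blackboard and sets speed and montages.
; Damage updates the HP bar, flashes the material and routes fire, ice or thunder types to effect components; death notifies the game mode.
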(event `Multi_SetPercent`
  (params (NewParam :type "Float (double-precision)"))
  ;[1 1 1] 멀티_SetPercent
  (bind _aswidget_monster_hp (cast `/Game/AI/Monster/Widget/Widget_MonsterHP` (`WidgetComponent.GetUserWidgetObject` (`self.Widget`))))
  (`ProgressBar.SetPercent` (`/Game/AI/Monster/Widget/Widget_MonsterHP.HP` _aswidget_monster_hp) NewParam))

(event `self.ReceiveBeginPlay`
  ;[1 1 1] Begin Play 이벤트
  (`/Engine/EditorBlueprintResources/ActorMacros.Switch Has Authority`
    (:`Authority`
      (`self.Server_Begin`))))

(event `Server_Begin`
  ;[1 1 1] Begin Play 이벤트
  (`self.SetState` "NewEnumerator0")
  (set `self.Offset` (`KismetMathLibrary.RandomFloatInRange` -7.0 7.0))
  (bind _returnvalue (`|GetDataTableRow` "/Game/AI/Monster/Struct/DT_Monster.DT_Monster" (`KismetStringLibrary.Conv_StringToName` (`KismetStringLibrary.Conv_IntToString` (`self.Level`))))
    (:`then`
      (bind (_maxhp _basicdamage _gold _start_movespeed _attackmontagecount) (break `/Game/AI/Monster/Struct/ST_Monster` _returnvalue))
      (set `self.MaxHP` _maxhp)
      (set `self.Damage` _basicdamage)
      (set `self.Gold` _gold)
      (set `self.CurrentSpeed` _start_movespeed)
      (set `self.Int_MaxAttackMontage` _attackmontagecount)
      (set `self.CurrentHP` (`self.MaxHP`))
      (bind _aswidget_monster_hp (cast `/Game/AI/Monster/Widget/Widget_MonsterHP` (`WidgetComponent.GetUserWidgetObject` (`self.Widget`))))
      (`/Engine/EditorBlueprintResources/StandardMacros.IsValid` _aswidget_monster_hp
        (:`Is Valid`
          (`self.Multi_SetPercent` (/ (`self.CurrentHP`) (`self.MaxHP`))))))))

(event `self.ReceiveAnyDamage`
  (params (Damage :type "Float (single-precision)") (DamageType :type "DamageType Object Reference") (InstigatedBy :type "Controller Object Reference") (DamageCauser :type "Actor Object Reference"))
  ;[1 1 1] AnyDamage 이벤트
  (`self.IsAlive`
    (:`True`
      (`|ExecutionSequence`
        (:`then_0`
          (`self.ProcessDamage` Damage)
          (`self.Multi_SetPercent` (/ (`self.CurrentHP`) (`self.MaxHP`)))
          (if (<= (`self.CurrentHP`) 0.0)
            (`self.Multi_SetPercent` (/ (`self.CurrentHP`) (`self.MaxHP`)))
            (bind _isdead (`self.CheckifDead`))
            (if _isdead
              (`self.OnDead` DamageCauser))
            (else
              (`self.ProcessSecondDamageByType` DamageType DamageCauser))))
        (:`then_1`
          (`self.Multi_Mat` (`self.SkeletalMesh`)))))))

(event `self.ReceiveTick`
  (params (DeltaSeconds :type "Float (single-precision)"))
  ;[1 1 1] Tick 이벤트
  (`/Engine/EditorBlueprintResources/ActorMacros.Switch Has Authority`
    (:`Authority`
      (`|ExecutionSequence`
        (:`then_0`
          (if (`|EnumEquality` (`self.CurrentState`) "NewEnumerator0")
            (`/Engine/EditorBlueprintResources/StandardMacros.IsValid` (`self.Spline_Ref`)
              (:`Is Valid`
                (`self.Server_TickMove`)))
            (else
              (set `self.B_PEACE_WALK` false))))
        (:`then_1`
          (if (`|EnumEquality` (`self.CurrentState`) "NewEnumerator6")
            (if (<= (`KismetMathLibrary.VSize` (- (`BlackboardComponent.GetValueAsVector` (`AIBlueprintHelperLibrary.GetBlackboard` null) (`self.Target`)) (`self.K2_GetActorLocation`))) 8.0)
              (`|PlayMontage` (`self.SkeletalMesh`) (`self.Run_Montage`) 1.0 0.0 "end"
                (:`then`
                  (`self.SetState` "NewEnumerator0"))))))))))

(event `OnDead`
  (params (DamageCauser :type "Actor Object Reference"))
  ;[1 1 1] 죽었을 때 실행되는 로직
  (`self.SetState` "NewEnumerator3")
  (`PrimitiveComponent.SetCollisionEnabled` (`self.CapsuleComponent`) "PhysicsOnly")
  (`|ExecutionSequence`
    (:`then_0`
      (bind _asbp_hero_base (cast `/Game/AI/Hero/BP_HERO_BASE` DamageCauser))
      (`KismetArrayLibrary.Array_RemoveItem` (`/Game/AI/Hero/BP_HERO_BASE.Monsters` _asbp_hero_base) self))
    (:`then_1`
      (`self.OnDeadPlayMontage`))))

(event `Server_TickMove`
  (bind _distancealongspline (`self.DistanceAlongSpline`))
  (bind _spline (`/Game/AI/Monster/Spline_Base.Spline` (`self.Spline_Ref`)))
  (bind (_returnvalue_x _returnvalue_y _returnvalue_z) (`KismetMathLibrary.BreakVector` (`SplineComponent.GetLocationAtDistanceAlongSpline` _spline _distancealongspline "World")))
  ;[1 1 1] Tick 이벤트
  (set `self.DistanceAlongSpline` (+ (* (* (`self.CurrentSpeed`) (`self.AxisValue`)) (`GameplayStatics.GetWorldDeltaSeconds`)) (`self.DistanceAlongSpline`)))
  (`self.K2_SetActorLocation` (`KismetMathLibrary.MakeVector` (+ (`self.Offset`) _returnvalue_x) (+ _returnvalue_y (`self.Offset`)) _returnvalue_z))
  (`self.K2_SetActorRelativeRotation` (`SplineComponent.GetRotationAtDistanceAlongSpline` _spline _distancealongspline "World"))
  (set `self.B_PEACE_WALK` true))

(event `ProcessSecondDamageByType`
  (params (DamageType :type "DamageType Object Reference") (DamageCauser :type "Actor Object Reference"))
  ;[1 1 1] AnyDamage 이벤트
  ;;[1 1 1] 2차 데미지 효과
  (bind _asbp_damage_base (cast `/Game/BluePrints/AllTower/MagicTower/DamageType/BP_DamageBase` DamageType))
  (switch `/Game/BluePrints/AllTower/MagicTower/DamageType/EAttackDamageType` (`/Game/BluePrints/AllTower/MagicTower/DamageType/BP_DamageBase.AttackDamageType` _asbp_damage_base)
    (:`NewEnumerator0`
      (`/Game/AI/Monster/BP_SecondDamageComponent.HandleDamage` (`self.BP_FireTypeComponent`) _asbp_damage_base DamageCauser :!label _label))
    (:`NewEnumerator1`
      (goto _label))
    (:`NewEnumerator6`
      (goto _label))
    (:`NewEnumerator2`
      (`/Game/AI/Monster/BP_SecondDamageComponent.HandleDamage` (`self.BP_IceTypeComponent`) _asbp_damage_base null :!label _label_2))
    (:`NewEnumerator3`
      (goto _label_2))
    (:`NewEnumerator7`
      (goto _label_2))
    (:`NewEnumerator4`
      (`ParticleSystemComponent.SetTemplate` (`self.ParticleSystem`) "/Game/GoodParticleStatus/Particles/Head_Status/PS_GPS_Stun.PS_GPS_Stun" :!label _label_3)
      (goto _label_2))
    (:`NewEnumerator5`
      (goto _label_3))
    (:`NewEnumerator8`
      (goto _label_3))))

(event `OnDeadPlayMontage`
  ;[1 1 1] 몬스터 사망시 몽타주 재생
  (`/Engine/EditorBlueprintResources/StandardMacros.IsValid` (`self.Die_Montage`)
    (:`Is Valid`
      (`GameplayStatics.PlaySoundAtLocation` (`self.DeadSound`) (`self.K2_GetActorLocation`) (struct) 1.0 1.0 0.0 null null null)
      (`|PlayMontage` (`self.SkeletalMesh`) (`self.Die_Montage`) 1.5 0.0 (`KismetStringLibrary.Conv_StringToName` (`KismetTextLibrary.Conv_TextToString` (`|FormatText` "Death{number}" (`KismetMathLibrary.RandomIntegerInRange` 1 (`self.Int_MaxDieMontage`)))))
        (:`then`
          (bind (_direction _power) (`Timeline|타임라인_2` :!via `PlayFromStart`)
            (:`Update`
              (`MeshComponent.SetScalarParameterValueOnMaterials` (`self.SkeletalMesh`) "Amount" _power))))
        (:`OnCompleted`
          (`self.DropGold`)
          (`self.CheckRemainingMonsterCount`))))))

(event `DropGold`
  ;[1 1 1] 몬스터 사망시 골드 드랍
  (`|SpawnActorFromClass` "/Game/AI/Mode/BP_Gold.BP_Gold_C" (`KismetMathLibrary.MakeTransform` (`self.K2_GetActorLocation`)) "Undefined" "OverrideRootScale" null (`self.Gold`) null)
  (`self.K2_DestroyActor`))

(event `SetState`
  (params (NewState :type "/Game/AI/Monster/BPE_MonsterState Enum" :default "NewEnumerator0"))
  (bind _returnvalue (`AIBlueprintHelperLibrary.GetBlackboard` (`self.GetController`)))
  ;[1 1 1] SetState 이벤트
  (if (`|EnumInequality` (`self.CurrentState`) "NewEnumerator3")
    (bind _output_get (set `self.CurrentState` NewState))
    (`|ExecutionSequence`
      (:`then_0`
        (`/Engine/EditorBlueprintResources/StandardMacros.IsValid` _returnvalue
          (:`Is Valid`
            (`BlackboardComponent.SetValueAsEnum` _returnvalue (`self.StateKey`) _output_get))))
      (:`then_1`
        (switch `/Game/AI/Monster/BPE_MonsterState` (`self.CurrentState`)
          (:`NewEnumerator0`
            (bind _output_get_2 (set `CharacterMovementComponent.MaxWalkSpeed` 5.0 (`self.CharacterMovement`)))
            (set `self.CurrentSpeed` _output_get_2))
          (:`NewEnumerator1`
            (bind _output_get_3 (set `CharacterMovementComponent.MaxWalkSpeed` 20.0 (`self.CharacterMovement`)))
            (set `self.CurrentSpeed` _output_get_3))
          (:`NewEnumerator2`
            (bind _output_get_4 (set `CharacterMovementComponent.MaxWalkSpeed` 1.0 (`self.CharacterMovement`)))
            (set `self.CurrentSpeed` _output_get_4)
            (`/Engine/EditorBlueprintResources/StandardMacros.IsValid` (`self.Attack_Montage`)
              (:`Is Valid`
                (`|PlayMontage` (`self.SkeletalMesh`) (`self.Attack_Montage`) 1.0 0.0 (`KismetStringLibrary.Conv_StringToName` (`KismetTextLibrary.Conv_TextToString` (`|FormatText` "Attack{Num}" (`KismetMathLibrary.RandomIntegerInRange` 1 (`self.Int_MaxAttackMontage`)))))
                  (:`OnCompleted`
                    (`self.AggroCheck`))))))
          (:`NewEnumerator3`
            (bind _output_get_5 (set `CharacterMovementComponent.MaxWalkSpeed` 0.0 (`self.CharacterMovement`)))
            (set `self.CurrentSpeed` _output_get_5))
          (:`NewEnumerator5`
            (bind _output_get_6 (set `CharacterMovementComponent.MaxWalkSpeed` 0.0 (`self.CharacterMovement`)))
            (set `self.CurrentSpeed` _output_get_6))
          (:`NewEnumerator6`
            (`|PlayMontage` (`self.SkeletalMesh`) (`self.Run_Montage`)
              (:`then`
                (set `CharacterMovementComponent.MaxWalkSpeed` 10.0 (`self.CharacterMovement`))))))))))

(event `CheckRemainingMonsterCount`
  ;[1 1 1] 남은 몬스터 수 확인
  (bind _asgm_hero_monster (cast `/Game/AI/GM_HeroMonster` (`GameplayStatics.GetGameMode`)))
  (`/Game/AI/GM_HeroMonster.CheckMonsterCount` _asgm_hero_monster))

(event `Multi_Mat`
  (params (NewParam :type "SkeletalMeshComponent Object Reference"))
  ;[1 1 1] 머티리얼 피격 효과 재생
  (`/Engine/EditorBlueprintResources/StandardMacros.IsValid` NewParam
    (:`Is Valid`
      (bind (_direction `_새_트랙_0`) (`Timeline|피격타임라인` :!via `PlayFromStart`)
        (:`Update`
          (`MeshComponent.SetScalarParameterValueOnMaterials` NewParam "OutlineEmissive" `_새_트랙_0`))))))

(event `self.PawnSensing.OnSeePawn`
  (params (Pawn :type "Pawn Object Reference"))
  (bind _targethero (`self.TargetHero`))
  ;[1 1 1] OnSeePawn 이벤트
  (bind _asbp_hero_base (cast `/Game/AI/Hero/BP_HERO_BASE` Pawn))
  (bind _currentstatepawn (`/Game/AI/Hero/BP_HERO_BASE.CurrentStatePawn` _asbp_hero_base))
  (if (and (`|EnumInequality` _currentstatepawn "NewEnumerator3") (`|EnumInequality` _currentstatepawn "NewEnumerator4"))
    (if (< (`KismetArrayLibrary.Array_Length` (`/Game/AI/Hero/BP_HERO_BASE.Monsters` _asbp_hero_base)) (`self.MaxBattelMonsterCount`))
      (set `self.DistanceToHero` 30.0)
      (set `self.TargetHero` null)
      (bind _outactors (`GameplayStatics.GetAllActorsOfClass` "/Game/AI/Hero/BP_HERO_BASE.BP_HERO_BASE_C"))
      (for _array_element _outactors
        (bind _returnvalue (`KismetMathLibrary.VSize` (- (`self.K2_GetActorLocation`) (`self.K2_GetActorLocation` _array_element))))
        (if (< _returnvalue (`self.DistanceToHero`))
          (set `self.DistanceToHero` _returnvalue)
          (set `self.TargetHero` _array_element)))
      (`/Engine/EditorBlueprintResources/StandardMacros.IsValid` _targethero
        (:`Is Valid`
          (bind _currentstatepawn_2 (`/Game/AI/Hero/BP_HERO_BASE.CurrentStatePawn` _array_element))
          (if (and (`|EnumInequality` _currentstatepawn_2 "NewEnumerator3") (`|EnumInequality` _currentstatepawn_2 "NewEnumerator4"))
            (set `self.Instigator` _targethero)
            (`self.SetState` "NewEnumerator1")
            (`GameplayStatics.PlaySoundAtLocation` (`self.ChaseSound`) (`self.K2_GetActorLocation`) (struct) 1.0 1.0 0.0 null null null)
            (`KismetArrayLibrary.Array_AddUnique` (`/Game/AI/Hero/BP_HERO_BASE.Monsters` _targethero) self)
            (`/Engine/EditorBlueprintResources/StandardMacros.DoOnce` false :!label _label_4
              (:`Completed`
                (`BlackboardComponent.SetValueAsVector` (`AIBlueprintHelperLibrary.GetBlackboard` (`AIBlueprintHelperLibrary.GetAIController` self)) (`self.Target`) (`self.K2_GetActorLocation`))))
            (else
              (set `self.DistanceToHero` 9999.0 :!label _label_5)
              (set `self.TargetHero` null))))
        (:`Is Not Valid`
          (goto _label_5))))))

(event `BasicAttack`
  (params (Damage :type "Float (double-precision)"))
  (bind _returnvalue (`self.K2_GetActorLocation`))
  ;[1 1 1] 몬스터 베이직 어택
  (bind _outactors (`GameplayStatics.GetAllActorsOfClass` "BP_Monster_BASIC_C"))
  (bind _outhit (`KismetSystemLibrary.CapsuleTraceSingleForObjects` _returnvalue (+ _returnvalue (* (`self.GetActorForwardVector`) 6.0)) 4.0 3.0 (`|MakeArray` "ObjectTypeQuery3" :!type "EObjectTypeQuery Enum") false _outactors "None" true (struct :`G` 0.207014 :`B` 1.0 :`A` 1.0) (struct :`R` 1.0 :`B` 0.951921 :`A` 1.0)))
  (bind _asbp_hero_base (cast `/Game/AI/Hero/BP_HERO_BASE` (`.HitActor` (`GameplayStatics.BreakHitResult` _outhit))))
  (`/Engine/EditorBlueprintResources/StandardMacros.IsValid` _asbp_hero_base
    (:`Is Valid`
      (`CharacterMovementComponent.AddImpulse` (`Character.CharacterMovement` _asbp_hero_base) (* (`self.GetActorForwardVector` _asbp_hero_base) -20.0) false)
      (`GameplayStatics.SpawnEmitterAtLocation` "/Game/SimpleCartoonFX/FX/Hit.Hit" (`self.K2_GetActorLocation` _asbp_hero_base) (struct) (0.05 0.05 0.05))
      (`GameplayStatics.ApplyDamage` _asbp_hero_base Damage null self))))

(event `Initi_TargetLoc`
  ;[1 1 1] OnSeePawn 이벤트
  (goto _label_4 :!via `Reset`))

(event `AggroCheck`
  (set `self.DistanceToHero` 99999.0)
  (set `self.TargetHero` null)
  (bind _outactors (`GameplayStatics.GetAllActorsOfClass` "/Game/AI/Hero/BP_HERO_BASE.BP_HERO_BASE_C"))
  (for _array_element _outactors
    (bind _returnvalue (`KismetMathLibrary.VSize` (- (`self.K2_GetActorLocation`) (`self.K2_GetActorLocation` _array_element))))
    (if (< _returnvalue (`self.DistanceToHero`))
      (set `self.DistanceToHero` _returnvalue)
      (set `self.TargetHero` _array_element)))
  (if (<= (`self.DistanceToHero`) 50.0)
    (set `self.Instigator` (`self.TargetHero`))
    (`self.SetState` "NewEnumerator1")
    (else
      (`self.SetState` "NewEnumerator0"))))

(event `Counter`
  (params (Hero :type "/Game/AI/Hero/BP_HERO_BASE Object Reference")))

(fn `CheckifDead`
  (returns (IsDead :type Boolean))
  (return (<= (`self.CurrentHP`) 0.0)))

(fn `ProcessDamage`
  (params (Damage :type "Float (double-precision)"))
  (set `self.CurrentHP` (- (`self.CurrentHP`) Damage)))

(fn `UpdateHPHud`
  (bind _aswidget_monster_hp (cast `/Game/AI/Monster/Widget/Widget_MonsterHP` (`WidgetComponent.GetUserWidgetObject` (`self.Widget`))))
  (`ProgressBar.SetPercent` (`/Game/AI/Monster/Widget/Widget_MonsterHP.HP` _aswidget_monster_hp) (/ (`self.CurrentHP`) (`self.MaxHP`))))

(fn `UserConstructionScript`
  (`parent.UserConstructionScript`))
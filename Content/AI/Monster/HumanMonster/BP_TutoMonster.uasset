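; BP_TutoMonster is a human monster variant, apparently for the tutorial, that walks a looping spline path with zero peripheral vision.
; In the first CurrentState value, Tick advances the distance by speed and axis value, snapping X, Y and rotation to the spline while keeping its own Z.
; BPEACEWALK is set during spline movement and cleared in other states.
; The distance resets to zero near the spline's end.
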(event `self.ReceiveBeginPlay`
  (`parent.ReceiveBeginPlay`)
  (set `self.StartLocation` (`self.K2_GetActorLocation`))
  (`PawnSensingComponent.SetPeripheralVisionAngle` (`self.PawnSensing`) 0.0))

(event `self.ReceiveTick`
  (params (DeltaSeconds :type "Float (single-precision)"))
  (bind (_returnvalue_x _returnvalue_y _returnvalue_z) (`KismetMathLibrary.BreakVector` (`self.K2_GetActorLocation`)))
  (bind _distancealongspline (`self.DistanceAlongSpline`))
  (bind _spline (`/Game/AI/Monster/Spline_Base_Tuto.Spline` (`self.Spline`)))
  (bind (_returnvalue_x_2 _returnvalue_y_2) (`KismetMathLibrary.BreakVector` (`SplineComponent.GetLocationAtDistanceAlongSpline` _spline _distancealongspline "World")))
  (if (`|EnumEquality` (`self.CurrentState`) "NewEnumerator0")
    (`/Engine/EditorBlueprintResources/StandardMacros.IsValid` (`self.Spline`)
      (:`Is Valid`
        (set `self.DistanceAlongSpline` (+ (* (* (`self.CurrentSpeed`) (`self.AxisValue`)) (`GameplayStatics.GetWorldDeltaSeconds`)) (`self.DistanceAlongSpline`)))
        (`self.K2_SetActorLocation` (`KismetMathLibrary.MakeVector` _returnvalue_x_2 _returnvalue_y_2 _returnvalue_z))
        (`self.K2_SetActorRelativeRotation` (`SplineComponent.GetRotationAtDistanceAlongSpline` _spline _distancealongspline "World"))
        (set `self.B_PEACE_WALK` true)
        (if (<= (- (`SplineComponent.GetSplineLength` (`/Game/AI/Monster/Spline_Base_Tuto.Spline` (`self.Spline`))) (`self.DistanceAlongSpline`)) 1.0)
          (set `self.DistanceAlongSpline` 0.0))))
    (else
      (set `self.B_PEACE_WALK` false))))

(fn `UserConstructionScript`
  (`parent.UserConstructionScript`))
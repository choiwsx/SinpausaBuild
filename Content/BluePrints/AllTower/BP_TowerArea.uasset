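; BP_TowerArea is a tower spot that shows a tower selection actor when a VR motion controller touches it.
; Mesh overlap calls a server event that flags the area and, gated by AreaSpawn and a DoOnce, spawns a tiny-scaled BP_TowerSelect at its location.
; Any end overlap clears the flag and, if a selection exists, destroys it and resets the gate.
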(event `SPAWN`
  (bind _returnvalue (`|SpawnActorFromClass` "/Game/BluePrints/AllTower/BP_TowerSelect.BP_TowerSelect_C" (`KismetMathLibrary.MakeTransform` (+ (`self.K2_GetActorLocation`) (0.0 0.0 0.0)) (struct) (0.01 0.01 0.01)) "Undefined" "OverrideRootScale" null null))
  (set `self.TowerSelected` _returnvalue))

(event `Server_TowerSelected`
  (set `self.AreaOverlap` true)
  (if (`self.AreaSpawn`)
    (goto _label :!via `Reset`)
    (else
      (`/Engine/EditorBlueprintResources/StandardMacros.DoOnce` false :!label _label
        (:`Completed`
          (`self.SPAWN`))))))

(event `self.StaticMesh.OnComponentBeginOverlap`
  (params (OverlappedComponent :type "PrimitiveComponent Object Reference") (OtherActor :type "Actor Object Reference") (OtherComp :type "PrimitiveComponent Object Reference") (OtherBodyIndex :type Integer) (bFromSweep :type Boolean) (SweepResult :type "HitResult Structure (by ref)"))
  (bind _asbp_motion_controller (cast `/Game/VirtualRealityBP/Blueprints/BP_MotionController` OtherActor))
  (`/Engine/EditorBlueprintResources/StandardMacros.IsValid` _asbp_motion_controller
    (:`Is Valid`
      (`self.Server_TowerSelected`))))

(event `Server_SetTowerSelected`
  (params (tower :type "/Game/BluePrints/AllTower/BP_TowerSelect Object Reference"))
  (set `self.TowerSelected` tower))

(event `self.StaticMesh.OnComponentEndOverlap`
  (params (OverlappedComponent :type "PrimitiveComponent Object Reference") (OtherActor :type "Actor Object Reference") (OtherComp :type "PrimitiveComponent Object Reference") (OtherBodyIndex :type Integer))
  (bind _towerselected (`self.TowerSelected`))
  (set `self.AreaOverlap` false)
  (`/Engine/EditorBlueprintResources/StandardMacros.IsValid` _towerselected
    (:`Is Valid`
      (`self.K2_DestroyActor` _towerselected)
      (goto _label :!via `Reset`))))

(fn `UserConstructionScript`)
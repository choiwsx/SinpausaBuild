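; BP_TowerAreaWonseok is a tower build spot that opens a build widget when a VR motion controller touches its box.
; The box overlap casts to BP_MotionController, stores it, and checks that its owning MotionControllerPawn is controlled by player controller 0.
; If that pawn is not already building, PC_Controller spawns the widget, receiving the motion controller, the static mesh's world transform and this area as tower base.
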(event `self.ReceiveBeginPlay`)

(event `self.Box.OnComponentBeginOverlap`
  (params (OverlappedComponent :type "PrimitiveComponent Object Reference") (OtherActor :type "Actor Object Reference") (OtherComp :type "PrimitiveComponent Object Reference") (OtherBodyIndex :type Integer) (bFromSweep :type Boolean) (SweepResult :type "HitResult Structure (by ref)"))
  (bind _returnvalue (`GameplayStatics.GetPlayerController` 0))
  (bind _asbp_motion_controller (cast `/Game/VirtualRealityBP/Blueprints/BP_MotionController` OtherActor))
  (set `self.MotionController` _asbp_motion_controller)
  (`/Engine/EditorBlueprintResources/StandardMacros.IsValid` _asbp_motion_controller
    (:`Is Valid`
      (bind _aspc_controller (cast `/Game/AI/PC_Controller` _returnvalue))
      (bind _asmotion_controller_pawn (cast `/Game/VirtualRealityBP/Blueprints/MotionControllerPawn` (`self.GetOwner` _asbp_motion_controller)))
      (if (== (`Pawn.GetController` _asmotion_controller_pawn) _returnvalue)
        (if (not (`/Game/VirtualRealityBP/Blueprints/MotionControllerPawn.IsBuilding?` _asmotion_controller_pawn))
          (`/Game/AI/PC_Controller.Spawn_BuildWidget` _aspc_controller _asbp_motion_controller (`SceneComponent.K2_GetComponentToWorld` (`self.StaticMesh`)) self null))))))

(fn `UserConstructionScript`)
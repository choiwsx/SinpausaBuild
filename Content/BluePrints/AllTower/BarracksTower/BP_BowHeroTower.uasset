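; BP_BowHeroTower is a barracks tower Blueprint that spawns and levels up a bow hero.
; On BeginPlay, the authority spawns a BP_BasicBow at a small offset from the tower through a server spawn event, passing the tower as its owner and storing it in Hero.
; LevelUPHero sets the BowHero reference to level 2 and calls its level-up function.
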(event `Server_Spawn`
  (params (NewParam :type "Transform Structure"))
  (`/Engine/EditorBlueprintResources/ActorMacros.Switch Has Authority`
    (:`Authority`
      (bind _returnvalue (`|SpawnActorFromClass` "/Game/AI/Hero/BP_BasicBow.BP_BasicBow_C" NewParam "AlwaysSpawn" "OverrideRootScale" null null null self null))
      (set `self.Hero` _returnvalue))))

(event `self.ReceiveBeginPlay`
  (`parent.ReceiveBeginPlay`)
  (`/Engine/EditorBlueprintResources/ActorMacros.Switch Has Authority`
    (:`Authority`
      (`self.Server_Spawn` (`KismetMathLibrary.MakeTransform` (+ (`self.K2_GetActorLocation`) (0.0 15.0 50.0)))))))

(event `LevelUPHero`
  (bind _bowhero (`self.BowHero`))
  (set `/Game/AI/Hero/BP_HERO_BASE.Level` 2 _bowhero)
  (`/Game/AI/Hero/BP_BasicSword.HeroLevelUp` _bowhero))

(event `self.ReceiveActorBeginOverlap`
  (params (OtherActor :type "Actor Object Reference"))
  (`parent.ReceiveActorBeginOverlap` OtherActor))

(fn `UserConstructionScript`
  (`parent.UserConstructionScript`))
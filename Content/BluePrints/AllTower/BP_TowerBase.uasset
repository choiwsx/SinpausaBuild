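; Base tower actor for a VR tower game that opens an upgrade option on controller touch and can fire at enemies.
; When a motion controller of the local player overlaps its Sphere and the pawn is not building, it asks PC_Controller to spawn the upgrade at the mesh transform.
; AttackEnemy1 spawns the tower type's attack actor at ShootingPoint with its damage, targeting the first listed enemy.
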(event `self.ReceiveBeginPlay`)

(event `self.Sphere.OnComponentBeginOverlap`
  (params (OverlappedComponent :type "PrimitiveComponent Object Reference") (OtherActor :type "Actor Object Reference") (OtherComp :type "PrimitiveComponent Object Reference") (OtherBodyIndex :type Integer) (bFromSweep :type Boolean) (SweepResult :type "HitResult Structure (by ref)"))
  (bind _returnvalue (`GameplayStatics.GetPlayerController` 0))
  (bind _asbp_motion_controller (cast `/Game/VirtualRealityBP/Blueprints/BP_MotionController` OtherActor))
  (set `self.MotionController` _asbp_motion_controller)
  (`/Engine/EditorBlueprintResources/StandardMacros.IsValid` _asbp_motion_controller
    (:`Is Valid`
      (bind _aspc_controller (cast `/Game/AI/PC_Controller` _returnvalue))
      (bind _asmotion_controller_pawn (cast `/Game/VirtualRealityBP/Blueprints/MotionControllerPawn` (`self.GetOwner` _asbp_motion_controller)))
      (if (== (`Pawn.GetController` _asmotion_controller_pawn) _returnvalue)
        (if (not (`/Game/VirtualRealityBP/Blueprints/MotionControllerPawn.IsBuilding?` _asmotion_controller_pawn))
          (`/Game/AI/PC_Controller.Spawn_Upgrade` _aspc_controller _asbp_motion_controller (`SceneComponent.K2_GetComponentToWorld` (`self.StaticMesh`)) self))))))

(fn `AttackEnemy1`
  (locals (NewLocalVar_0 :type "/Game/HR/BP_HRBulletBase Object Reference"))
  (bind _listofenemy (`self.ListOfEnemy`))
  (bind (_towernumber _towername _towerattackdelay _towerdamage _towerange _towerselection _attacktype) (break `/Game/HR/BP_HRStruct` (`self.Tower종류`)))
  (if (!= (`KismetArrayLibrary.Array_Length` _listofenemy) 0)
    (bind _returnvalue (`|SpawnActorFromClass` _attacktype (`SceneComponent.K2_GetComponentToWorld` (`self.Shooting Point`)) "AlwaysSpawn" "OverrideRootScale" null _towerdamage null))
    (`/Engine/EditorBlueprintResources/StandardMacros.IsValid` null
      (:`Is Valid`
        (set `/Game/HR/BP_HRBulletBase.EnemyToAttack` (`|GetArrayItem` _listofenemy) _returnvalue)))))

(fn `UserConstructionScript`)
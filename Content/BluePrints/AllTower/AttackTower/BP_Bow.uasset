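; BP_Bow is the attack unit of an arrow tower that shoots at monsters and destroys itself once its ArrowTower is gone.
; Sphere overlap adds monsters to an Enemy list and starts a looping attack timer.
; Each tick of that timer rotates toward the nearest listed monster within a hardcoded XY radius and spawns BP_Arrow with data-table damage, muzzle effect and sound.
; End overlap is empty, so the list is never pruned.
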(event `Rotate`
  (params (NewParam :type "/Game/AI/Monster/BP_Monster_BASIC Object Reference"))
  (bind (_returnvalue_roll _returnvalue_pitch _returnvalue_yaw) (`KismetMathLibrary.BreakRotator` (`KismetMathLibrary.FindLookAtRotation` (`self.K2_GetActorLocation`) (`self.K2_GetActorLocation` NewParam))))
  ;[1 1 1] 회전함수
  (`/Engine/EditorBlueprintResources/StandardMacros.IsValid` NewParam
    (:`Is Valid`
      (`self.K2_SetActorRotation` (`KismetMathLibrary.MakeRotator` 0.0 _returnvalue_pitch _returnvalue_yaw)))))

(event `ArrowSpawn`
  (bind _bow (`self.Bow`))
  (bind _returnvalue (`SceneComponent.GetSocketLocation` _bow "hand_lBowSocket"))
  ;[1 1 1] 화살 발사
  (cast `/Game/AI/PC_Controller` (`GameplayStatics.GetPlayerController` 0))
  (`GameplayStatics.SpawnEmitterAtLocation` "/Game/GabrielAguiarProd/ToonProjectilesVol1/Particles/Muzzles/P_Muzzle_Bullet01Lowpoly.P_Muzzle_Bullet01Lowpoly" (`SceneComponent.GetSocketLocation` _bow "hand_lBowSocket") (`self.K2_GetActorRotation`) (0.05 0.05 0.05))
  (bind _returnvalue_2 (`|GetDataTableRow` "/Game/HR/BP_HRDataTable.BP_HRDataTable" (`self.StructRow`))
    (:`then`
      (`|SpawnActorFromClass` "/Game/BluePrints/AllTower/AttackTower/BP_Arrow.BP_Arrow_C" (`KismetMathLibrary.MakeTransform` _returnvalue (`self.K2_GetActorRotation`)) "AlwaysSpawn" "OverrideRootScale" self (`.TowerDamage_19_4DB1C961479B2BC080C0E1A9A0B59899` (break `/Game/HR/BP_HRStruct` _returnvalue_2)) null)
      (`GameplayStatics.PlaySoundAtLocation` "/Game/Sound/Using/TowerAttackSound/Arrow_Impact_flesh__human__8.Arrow_Impact_flesh__human__8" _returnvalue (struct) 1.0 1.0 0.0 null null null)
      (`KismetSystemLibrary.Delay` 0.5))))

(event `self.ReceiveTick`
  (params (DeltaSeconds :type "Float (single-precision)"))
  ;[1 1 1] 타워가 삭제되면 공격유닛도 삭제
  (`/Engine/EditorBlueprintResources/StandardMacros.IsValid` (`self.ArrowTower`)
    (:`Is Not Valid`
      (`self.K2_DestroyActor`))))

(event `self.Sphere.OnComponentBeginOverlap`
  (params (OverlappedComponent :type "PrimitiveComponent Object Reference") (OtherActor :type "Actor Object Reference") (OtherComp :type "PrimitiveComponent Object Reference") (OtherBodyIndex :type Integer) (bFromSweep :type Boolean) (SweepResult :type "HitResult Structure (by ref)"))
  (bind _asbp_monster_basic (cast `/Game/AI/Monster/BP_Monster_BASIC` OtherActor)) ; 회전을 하면됨
  (`KismetArrayLibrary.Array_AddUnique` (`self.Enemy`) _asbp_monster_basic)
  (if (not (`KismetSystemLibrary.K2_IsTimerActiveHandle` (`self.TimeEvent_Attack`)))
    (`self.CheckAndAttack`)))

(event `CheckAndAttack`
  (bind _returnvalue (`KismetSystemLibrary.K2_SetTimerDelegate` (delegate `CheckAndAttack_Timer`) (`self.AttackSpeed`) true))
  (set `self.TimeEvent_Attack` _returnvalue))

(event `CheckAndAttack_Timer`
  (bind _targetmonster (`self.TargetMonster`))
  (set `self.DistanceToMonster` 30.0)
  (set `self.TargetMonster` null)
  (for _array_element (`self.Enemy`)
    (`/Engine/EditorBlueprintResources/StandardMacros.IsValid` _array_element
      (:`Is Valid`
        (bind _returnvalue (`KismetMathLibrary.VSizeXY` (- (`self.K2_GetActorLocation` _array_element) (`self.K2_GetActorLocation`))))
        (if (< _returnvalue (`self.DistanceToMonster`))
          (set `self.DistanceToMonster` _returnvalue)
          (set `self.TargetMonster` _array_element)))))
  (`/Engine/EditorBlueprintResources/StandardMacros.IsValid` _targetmonster
    (:`Is Valid`
      (`self.Rotate` _targetmonster)
      (`self.ArrowSpawn`)
      (if (== (`KismetArrayLibrary.Array_Length` (`self.Enemy`)) 0)
        (`KismetSystemLibrary.K2_ClearAndInvalidateTimerHandle` (`self.TimeEvent_Attack`))))))

(event `self.Sphere.OnComponentEndOverlap`
  (params (OverlappedComponent :type "PrimitiveComponent Object Reference") (OtherActor :type "Actor Object Reference") (OtherComp :type "PrimitiveComponent Object Reference") (OtherBodyIndex :type Integer)))

(fn `CheckNewTarget`)

(fn `CheckTargetCalculation`
  (params (In :type "Array of HitResult Structure"))
  (locals (TempDistance :type "Float (double-precision)" :default 0.0) (TempTarget :type "/Game/AI/Monster/BP_Monster_BASIC Object Reference")))

(fn `UserConstructionScript`)
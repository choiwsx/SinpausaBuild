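; Level 2 cannon tower for a tower game played with motion controllers.
; On BeginPlay it reads its row from BP_HRDataTable and spawns a scaled BP_Cannon just above itself, passing the row, itself and the attack delay.
; When a motion controller of the first local player overlaps its Sphere outside build mode, it calls Level2towerSell on PC_Controller with the controller, mesh transform and tower.
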(event `self.ReceiveBeginPlay`
  (`parent.ReceiveBeginPlay`)
  (bind _returnvalue (`|GetDataTableRow` "/Game/HR/BP_HRDataTable.BP_HRDataTable" "8")
    (:`then`
      (`|SpawnActorFromClass` "/Game/BluePrints/AllTower/AttackTower/BP_Cannon.BP_Cannon_C" (`KismetMathLibrary.MakeTransform` (+ (`self.K2_GetActorLocation`) (0.35 0.0 10.0)) (struct) (0.8 0.8 0.8)) "Undefined" "OverrideRootScale" null "8" self (`.TowerAttackDelay_47_A8719F8E4CCD328B3B8027A0E52B601F` (break `/Game/HR/BP_HRStruct` _returnvalue)) null))))

(event `self.Sphere.OnComponentBeginOverlap`
  (params (OverlappedComponent :type "PrimitiveComponent Object Reference") (OtherActor :type "Actor Object Reference") (OtherComp :type "PrimitiveComponent Object Reference") (OtherBodyIndex :type Integer) (bFromSweep :type Boolean) (SweepResult :type "HitResult Structure (by ref)"))
  (bind _returnvalue (`GameplayStatics.GetPlayerController` 0))
  (bind _asbp_motion_controller (cast `/Game/VirtualRealityBP/Blueprints/BP_MotionController` OtherActor))
  (set `self.MotionController` _asbp_motion_controller)
  (`/Engine/EditorBlueprintResources/StandardMacros.IsValid` _asbp_motion_controller
    (:`Is Valid`
      (bind _aspc_controller (cast `/Game/AI/PC_Controller` _returnvalue))
      (bind _asmotion_controller_pawn (cast `/Game/VirtualRealityBP/Blueprints/MotionControllerPawn` (`self.GetOwner` _asbp_motion_controller)))
      (if (== (`Pawn.GetController` _asmotion_controller_pawn) _returnvalue)
        (if (not (`/Game/VirtualRealityBP/Blueprints/MotionControllerPawn.IsBuilding?` _asmotion_controller_pawn))
          (`/Game/AI/PC_Controller.Level2towerSell` _aspc_controller (`self.MotionController`) (`SceneComponent.K2_GetComponentToWorld` (`self.StaticMesh`)) self))))))

(fn `UserConstructionScript`
  (`parent.UserConstructionScript`))
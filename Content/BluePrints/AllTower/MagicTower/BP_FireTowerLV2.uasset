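; BP_FireTowerLV2 is a level 2 fire magic tower in a motion-controller game.
; Tick, gated by a Make flag and a one-second Delay, spawns one small BP_Fire above the tower with itself as owner tower.
; When the local player's motion controller overlaps its Sphere outside building mode, it calls PC_Controller's Level2towerSell with the controller, mesh transform and tower.
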(event `self.ReceiveTick`
  (params (DeltaSeconds :type "Float (single-precision)"))
  (if (not (`self.Make`))
    (`KismetSystemLibrary.Delay` 1.0)
    (`|SpawnActorFromClass` "/Game/BluePrints/AllTower/MagicTower/BP_Fire.BP_Fire_C" (`KismetMathLibrary.MakeTransform` (+ (`self.K2_GetActorLocation`) (0.0 0.0 35.0)) (struct) (0.02 0.02 0.02)) "Undefined" "OverrideRootScale" null self "9" null)
    (set `self.Make` true)))

(event `self.ReceiveBeginPlay`
  (set `self.Make` false))

(event `self.Sphere.OnComponentBeginOverlap`
  (params (OverlappedComponent :type "PrimitiveComponent Object Reference") (OtherActor :type "Actor Object Reference") (OtherComp :type "PrimitiveComponent Object Reference") (OtherBodyIndex :type Integer) (bFromSweep :type Boolean) (SweepResult :type "HitResult Structure (by ref)"))
  (bind _returnvalue (`GameplayStatics.GetPlayerController` 0))
  (bind _asbp_motion_controller (cast `/Game/VirtualRealityBP/Blueprints/BP_MotionController` OtherActor))
  (set `self.MotionController` _asbp_motion_controller)
  (`/Engine/EditorBlueprintResources/StandardMacros.IsValid` _asbp_motion_controller
    (:`Is Valid`
      (bind _aspc_controller (cast `/Game/AI/PC_Controller` _returnvalue))
      (bind _asmotion_controller_pawn (cast `/Game/VirtualRealityBP/Blueprints/MotionControllerPawn` (`self.GetOwner` _asbp_motion_controller)))
      (if (== (`Pawn.GetController` _asmotion_controller_pawn) _returnvalue)
        (if (not (`/Game/VirtualRealityBP/Blueprints/MotionControllerPawn.IsBuilding?` _asmotion_controller_pawn))
          (`/Game/AI/PC_Controller.Level2towerSell` _aspc_controller (`self.MotionController`) (`SceneComponent.K2_GetComponentToWorld` (`self.StaticMesh`)) self))))))

(fn `UserConstructionScript`
  (`parent.UserConstructionScript`))
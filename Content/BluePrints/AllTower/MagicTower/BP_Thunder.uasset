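; BP_Thunder is a magic tower's lightning projectile that grows until ready, then falls under gravity when dropped.
; Tick scales it up with collision off until target size, then marks the Tower ready, or destroys it if the Tower is invalid.
; On hit, it spawns lightning and sound, clears the Tower's flags, destroys itself and applies data-table-driven radial damage that ignores heroes.
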(event `self.Drop`
  ;[1 1 1] Drop
  (`parent.Drop`)
  (`PrimitiveComponent.SetEnableGravity` (`self.Mesh`) true))

(event `self.ReceiveTick`
  (params (DeltaSeconds :type "Float (single-precision)"))
  (bind _tower (`self.Tower`))
  ;[1 1 1] 불 생성
  (`/Engine/EditorBlueprintResources/StandardMacros.IsValid` _tower
    (:`Is Valid`
      (if (not (`/Game/BluePrints/AllTower/BP_TowerBase.Ready` _tower))
        (`self.Grow`)))
    (:`Is Not Valid`
      (`self.K2_DestroyActor`))))

(event `self.ReceiveHit`
  (params (MyComp :type "PrimitiveComponent Object Reference") (Other :type "Actor Object Reference") (OtherComp :type "PrimitiveComponent Object Reference") (bSelfMoved :type Boolean) (HitLocation :type "Vector Structure") (HitNormal :type "Vector Structure") (NormalImpulse :type "Vector Structure") (Hit :type "HitResult Structure (by ref)"))
  ;[1 1 1] 데미지
  (bind _outactors (`GameplayStatics.GetAllActorsOfClass` "/Game/AI/Hero/BP_HERO_BASE.BP_HERO_BASE_C"))
  (set `self.Hero_Array` _outactors)
  (`self.MagicEffect` HitLocation)
  (`self.MagicDamage` HitLocation))

(event `MagicDamage`
  (params (DamageLocation :type "Vector Structure"))
  ;[1 1 1] 마법 데미지
  (cast `/Game/AI/PC_Controller` (`GameplayStatics.GetPlayerController` 0))
  (bind _returnvalue (`|GetDataTableRow` "/Game/HR/BP_HRDataTable.BP_HRDataTable" (`self.TowerStruct`))
    (:`then`
      (bind (_towernumber _towername _towerattackdelay _towerdamage _towerange _towerselection _attacktype _magictype) (break `/Game/HR/BP_HRStruct` _returnvalue))
      (`GameplayStatics.ApplyRadialDamage` _towerdamage DamageLocation 25.0 _magictype (`self.Hero_Array`) self null true))))

(event `MagicEffect`
  (params (EffectLocation :type "Vector Structure"))
  (bind _tower (`self.Tower`))
  ;[1 1 1] 마법 이펙트
  (`GameplayStatics.SpawnEmitterAtLocation` "/Game/Luos4elements2/Particles/Lightning/Par_4E_LightningStrike_01.Par_4E_LightningStrike_01" EffectLocation (struct) (0.08 0.08 0.1))
  (set `/Game/BluePrints/AllTower/BP_TowerBase.Make` false _tower)
  (`self.K2_DestroyActor`)
  (set `/Game/BluePrints/AllTower/BP_TowerBase.Ready` false _tower)
  (`GameplayStatics.PlaySoundAtLocation` "/Game/Sound/Using/MagicSound/ElectricImpact1.ElectricImpact1" EffectLocation (struct) 0.5 1.0 0.0 null null null))

(event `Grow`
  ;[1 1 1] 마법 크게 변환
  (`self.SetActorEnableCollision` false)
  (`self.SetActorScale3D` (+ (`self.GetActorScale3D`) (0.0001 0.0001 0.0001)))
  (if (== (`self.GetActorScale3D`) (0.1 0.1 0.1) :`ErrorTolerance` 1e-05)
    (`GameplayStatics.PlaySoundAtLocation` "/Game/Sound/Using/MagicSound/Collect_star_1.Collect_star_1" (0.0 0.0 0.0) (struct) 1.0 1.0 0.0 null null null)
    (set `/Game/BluePrints/AllTower/BP_TowerBase.Ready` true (`self.Tower`))
    (`self.SetActorEnableCollision` true)))

(fn `UserConstructionScript`
  (`parent.UserConstructionScript`))
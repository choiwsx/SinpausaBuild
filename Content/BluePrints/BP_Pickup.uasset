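; BP_Pickup is a pickup actor that replaces itself with a fresh copy when dropped.
; BeginPlay caches the starting location for later respawning.
; Drop runs the parent logic, destroys the actor, and plays a gold-gain particle and click sound at its current position.
; It then immediately spawns a new BP_Pickup at the cached location with a fixed rotation.
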(event `/Game/VirtualRealityBP/Blueprints/PickupActorInterface.Drop`
  (`parent.Drop`)
  (`self.K2_DestroyActor`)
  (`GameplayStatics.SpawnEmitterAtLocation` "/Game/GabrielAguiarProd/ToonProjectilesVol1/Particles/Muzzles/P_GainGold.P_GainGold" (`self.K2_GetActorLocation`) (struct) (0.5 0.5 0.5))
  (`GameplayStatics.PlaySoundAtLocation` "/Game/Sound/Using/GameEffectSound/Fantasy_click_sounds_2.Fantasy_click_sounds_2" (`self.K2_GetActorLocation`) (struct) 1.0 1.0 0.0 null null null)
  (`|SpawnActorFromClass` "BP_Pickup_C" (`KismetMathLibrary.MakeTransform` (`self.Location`) (struct :`Pitch` 90.0 :`Yaw` 180.0 :`Roll` 180.0)) "Undefined" "OverrideRootScale" null null))

(event `self.ReceiveBeginPlay`
  (`parent.ReceiveBeginPlay`)
  (set `self.Location` (`self.K2_GetActorLocation`)))

(fn `UserConstructionScript`
  (`parent.UserConstructionScript`))